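; BP_HealthPickUp is a pickup actor that heals any BP_CharacterBase that overlaps it.
; On overlap it adds HealAmount to the character's Health, capped at the class default Health, which serves as the maximum.
; It destroys itself after healing and stays in place if Health already equals that default.
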(event Collision|EventActorBeginOverlap
  (params (OtherActor :type Actor%20Object%20Reference))
  (bind _asbp_character_base (Utilities|Casting|CastToBP_CharacterBase OtherActor))
  (if (not (== (Variables|/Game/Blueprints/BP_CharacterBase.BP_CharacterBase_C|GetHealth _asbp_character_base) (.Health (Utilities|GetClassDefaults (Utilities|GetClass _asbp_character_base)))))
    (Variables|/Game/Blueprints/BP_CharacterBase.BP_CharacterBase_C|SetHealth _asbp_character_base (Math|Float|Min(Float) (+ (Variables|/Game/Blueprints/BP_CharacterBase.BP_CharacterBase_C|GetHealth _asbp_character_base) (Variables|Default|GetHealAmount)) (.Health (Utilities|GetClassDefaults (Utilities|GetClass _asbp_character_base)))))
    (Actor|DestroyActor)))

(fn ConstructionScript)