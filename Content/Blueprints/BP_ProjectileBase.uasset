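; BP_ProjectileBase is a projectile actor, named as a base class, that damages characters it overlaps.
; On overlap it casts to BP_CharacterBase, skips its own Instigator, applies fixed damage credited to the Instigator's controller, then destroys itself.
; Overlaps with other actor types are ignored.
; The Destroyed event spawns the P_Impulse emitter at its location, so the effect plays however the projectile is destroyed.
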(event Collision|EventActorBeginOverlap
  (params (OtherActor :type Actor%20Object%20Reference))
  (bind _instigator (Variables|Actor|GetInstigator))
  (bind _asbp_character_base (Utilities|Casting|CastToBP_CharacterBase OtherActor))
  (if (not (== _asbp_character_base _instigator))
    (Game|Damage|ApplyDamage _asbp_character_base 5e+01 (Pawn|GetController _instigator) self)
    (Actor|DestroyActor)))

(event EventDestroyed
  (Effects|SpawnEmitteratLocation "/Game/Assets/FX/P_Impulse.P_Impulse" (Transformation|GetActorLocation)))

(fn ConstructionScript)