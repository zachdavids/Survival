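; Game mode that runs wave-based enemy spawning from the Waves array.
; Each wave's class list is copied into Queue and shuffled, then a looping one-second timer spawns the front entry at random PlayerStart actors.
; When a spawned enemy is destroyed, an empty queue and no remaining BP_AIControllerBase actors trigger the next wave.
; WaveIndex increments without a bounds check on the last wave.
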(event Custom|SpawnEnemy
  (if (> (Utilities|Array|Length (Variables|Default|GetQueue)) 0)
    (bind _outactors (Actor|GetAllActorsOfClass "/Script/Engine.PlayerStart"))
    (bind _returnvalue (AI|SpawnAIFromClass (Utilities|Array|Get(acopy) (Variables|Default|GetQueue)) 0 (.location (Transformation|GetActorTransform (Utilities|Array|Get(acopy) _outactors (Math|Random|RandomInteger (Utilities|Array|Length _outactors))))) (.rotation (Transformation|GetActorTransform (Utilities|Array|Get(acopy) _outactors (Math|Random|RandomInteger (Utilities|Array|Length _outactors))))) false))
    (Utilities|Array|RemoveIndex (Variables|Default|GetQueue))
    (Game|BindEventtoOnDestroyed _returnvalue (delegate Custom|CheckWaveComplete))))

(event Custom|StartNewWave
  (Math|Integer|IncrementInt (Variables|Default|GetWaveIndex)
    (:%20%20
      (bind _output_get (Variables|Default|SetQueue (.classtospawn (Utilities|Array|Get(acopy) (Variables|Default|GetWaves) (Variables|Default|GetWaveIndex)))))
      (Utilities|Array|Shuffle _output_get))))

(event Custom|CheckWaveComplete
  (params (DestroyedActor :type Actor%20Object%20Reference))
  (if (== (Utilities|Array|Length (Variables|Default|GetQueue)) 0)
    (bind _outactors (Actor|GetAllActorsOfClass "/Game/Blueprints/BP_AIControllerBase.BP_AIControllerBase_C"))
    (if (== (Utilities|Array|Length _outactors) 0)
      (CallFunction|StartNewWave))))

(event Custom|ResetGame
  (Variables|Default|SetWaveIndex 0)
  (bind _output_get (Variables|Default|SetQueue (.classtospawn (Utilities|Array|Get(acopy) (Variables|Default|GetWaves) (Variables|Default|GetWaveIndex)))))
  (Utilities|Array|Shuffle _output_get))

(event EventBeginPlay
  (Utilities|Time|SetTimerbyEvent (delegate Custom|SpawnEnemy) 1.0 true)
  (CallFunction|ResetGame))

(fn ConstructionScript)